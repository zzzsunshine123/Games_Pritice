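; Arcane Shards gameplay ability that erupts a series of damaging shards around a targeted ground point.
; It shows a magic circle until input, then plays a cast montage whose event captures the mouse location.
; A spawned BP_PointCollection supplies randomly rotated ground points, their count scaling with ability level up to a cap.
; A looping timer visits each point, committing the ability, applying radial damage with outward knockback and firing a GameplayCue.
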(event `self.K2_ActivateAbility`
  (`|ExecutionSequence`
    (:`then_0`
      (message `PlayerInterface.ShowMagicCircle` (`self.GetAvatarActorFromActorInfo`) null))
    (:`then_1`
      (`AbilityTask_WaitInputPress.WaitInputPress` false
        (:`OnPress`
          (`|ExecutionSequence`
            (:`then_0`
              (`AbilityTask_PlayMontageAndWait.CreatePlayMontageAndWaitProxy` "None" "/Game/Assets/Characters/Aura/Animations/Abilities/AM_Cast_ArcaneShards.AM_Cast_ArcaneShards"
                (:`then`
                  (`AbilityTask_WaitGameplayEvent.WaitGameplayEvent` (struct :`TagName` "Event.Montage.ArcaneShard") null true
                    (:`then`
                      (bind (_asynctaskproxy _datahandle) (`TargetDataUnderMouse.CreateTargetDataUnderMouse`)
                        (:`VaildData`
                          (set `self.MouseHitLocation` (`.ImpactPoint` (`GameplayStatics.BreakHitResult` (`AbilitySystemBlueprintLibrary.GetHitResultFromTargetData` _datahandle))))
                          (bind _returnvalue (`|SpawnActorFromClass` "/Game/Blueprints/AbilitySystem/Aura/Abilities/Arcane/ArcaneShards/BP_PointCollection.BP_PointCollection_C" (`KismetMathLibrary.MakeTransform` (`self.MouseHitLocation`)) "AlwaysSpawn" "MultiplyWithRoot" null null))
                          (bind _output_get (set `self.BP_PointCollection` _returnvalue))
                          (set `self.PointCollection` _output_get)
                          (set `self.Num Points` (`KismetMathLibrary.Min` (`self.GetAbilityLevel`) (`self.MaxNumPoints`)))
                          (set `self.PointArray` (`PointCollection.GetGroundPoints` (`self.BP_PointCollection`) (`self.MouseHitLocation`) (`self.Num Points`) (`KismetMathLibrary.RandomFloatInRange` 0.0 360.0)))
                          (bind _returnvalue_2 (`KismetSystemLibrary.K2_SetTimerDelegate` (delegate `SpawnShard`) (`self.ShardSpawnDeltaTime`) true))
                          (set `self.ShardSpawnTimer` _returnvalue_2)
                          (message `PlayerInterface.HideMagicCircle` (`self.GetAvatarActorFromActorInfo`)))))))))
            (:`then_1`
              (message `CombatInterface.UpdateFacingTarget` (`self.GetAvatarActorFromActorInfo`) (`self.MouseHitLocation`)))))))))

(event `SpawnShard`
  (bind _returnvalue (`self.GetAvatarActorFromActorInfo`))
  (if (< (`self.Count`) (`self.Num Points`))
    (set `self.PointLocation` (`SceneComponent.K2_GetComponentLocation` (`|GetArrayItem` (`self.PointArray`) (`self.Count`))))
    (bind _outoverlappingactors (`AuraAbilitySystemLibrary.GetLivePlayersWithinRadius` _returnvalue (`|MakeArray` _returnvalue) (`self.RadialDamageOuterRadius`) (`self.PointLocation`)))
    (bind _output_get (set `self.Overlaped Enemy` _outoverlappingactors))
    (`self.K2_CommitAbility`)
    (for _array_element _output_get
      (bind _returnvalue_2 (- (`Actor.K2_GetActorLocation` _array_element) (`self.PointLocation`)))
      (`AuraAbilitySystemLibrary.ApplyDamageEffect` (`self.MakeDamageEffectParamsFromClassDefaults` _array_element (`self.PointLocation`) true _returnvalue_2 true _returnvalue_2 true)))
    (set `self.Count` (+ (`self.Count`) 1))
    (`self.K2_ExecuteGameplayCueWithParams` (struct :`TagName` "GameplayCue.ArcaneShards") (`AbilitySystemBlueprintLibrary.MakeGameplayCueParameters` 0.0 0.0 (struct) (struct) (struct) (struct) (struct) (`self.PointLocation`)))
    (else
      (`KismetSystemLibrary.K2_ClearAndInvalidateTimerHandle` (`self.ShardSpawnTimer`))
      (`KismetSystemLibrary.Delay` 0.2)
      (`Actor.K2_DestroyActor` (`self.PointCollection`))
      (`self.K2_EndAbility`))))