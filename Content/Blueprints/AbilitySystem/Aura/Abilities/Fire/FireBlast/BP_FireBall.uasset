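; Fire Blast fireball projectile that flies out and returns like a boomerang, exploding near its return actor.
; On the server, an outgoing timeline lerps it forward to an apex, then a returning timeline lerps it toward that actor's current location.
; Within explode distance, it calls OnHit, applies radial damage with outward knockback and death impulse to nearby live players except its owner, then destroys itself.
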(event `self.StartOutgoingTimeline`
  (bind _array (`|MakeArray` (`self.GetOwner`)))
  (`/Engine/EditorBlueprintResources/ActorMacros.Switch Has Authority`
    (:`Authority`
      (set `self.InitLocation` (`self.K2_GetActorLocation`))
      (set `self.ApexLocation` (+ (`self.InitLocation`) (* (`self.GetActorForwardVector`) (`self.TravelDistance`))))
      (bind (_direction _outgoingtrack) (`Timeline|OutgoingTimeline`)
        (:`Update`
          (`self.K2_SetActorLocation` (`KismetMathLibrary.VLerp` (`self.InitLocation`) (`self.ApexLocation`) _outgoingtrack)))
        (:`Finished`
          (bind (_direction_2 _returing_track) (`Timeline|Returning Timeline`)
            (:`Update`
              (`self.K2_SetActorLocation` (`KismetMathLibrary.VLerp` (`self.ApexLocation`) (`self.K2_GetActorLocation` (`self.ReturnToActor`)) _returing_track))
              (if (`self.IsWithinExplodeDistance`)
                (`self.OnHit`)
                (`KismetArrayLibrary.Array_Add` _array self)
                (bind _outoverlappingactors (`AuraAbilitySystemLibrary.GetLivePlayersWithinRadius` self _array 100.0 (`self.K2_GetActorLocation`)))
                (set `self.OverlapingEnemies` _outoverlappingactors)
                (`AuraAbilitySystemLibrary.SetIsRadialDamageEffectParam` (`self.ExplosionDamageParams`) true 50.0 100.0 (`self.K2_GetActorLocation`))
                (for _array_element (`self.OverlapingEnemies`)
                  (`AuraAbilitySystemLibrary.SetTargetEffectParamsASC` (`self.ExplosionDamageParams`) (`AbilitySystemBlueprintLibrary.GetAbilitySystemComponent` _array_element))
                  (bind _returnvalue (- (`self.K2_GetActorLocation` _array_element) (`self.K2_GetActorLocation`)))
                  (`AuraAbilitySystemLibrary.SetKnockbackDirection` (`self.ExplosionDamageParams`) _returnvalue 800.0)
                  (`AuraAbilitySystemLibrary.SetDeathImpulseDirection` (`self.ExplosionDamageParams`) _returnvalue 800.0)
                  (`AuraAbilitySystemLibrary.ApplyDamageEffect` (`self.ExplosionDamageParams`)))
                (`self.K2_DestroyActor`)))))))))

(fn `IsWithinExplodeDistance`
  (returns (ReturnValue :type Boolean))
  (return (<= (`KismetMathLibrary.VSize` (- (`self.K2_GetActorLocation`) (`self.K2_GetActorLocation` (`self.ReturnToActor`)))) (`self.ExplodeDistance`))))

(fn `UserConstructionScript`)