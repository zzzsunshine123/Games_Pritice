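; Enemy melee attack ability that faces the combat target, plays a random tagged montage and damages nearby hostile players.
; It waits for the montage's gameplay event, then runs a radius query at the tagged combat socket, drawing a debug sphere.
; Any hit fires the MeleeAttack gameplay cue with the montage tag and socket location.
; The ability ends after the event or when the montage finishes or stops.
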(event `self.K2_ActivateAbility`
  (bind _returnvalue (`self.GetAvatarActorFromActorInfo`))
  (bind _returnvalue_2 (`self.GetAvatarActorFromActorInfo`))
  (set `self.HasHitTarget` false)
  (set `self.DebugLocation` (`Actor.K2_GetActorLocation` _returnvalue))
  (bind _returnvalue_3 (message `EnemyInterface.GetCombatTarget` _returnvalue))
  (message `CombatInterface.UpdateFacingTarget` _returnvalue (`Actor.K2_GetActorLocation` _returnvalue_3))
  (bind _returnvalue_4 (message `CombatInterface.GetAttackMontages` (`self.GetAvatarActorFromActorInfo`)))
  (bind _returnvalue_5 (`self.GetRandomTaggedMontageFromArray` _returnvalue_4))
  (set `self.TagMontage` _returnvalue_5)
  (bind (_montage _montagetag _sockettag) (break `TaggedMontage` _returnvalue_5))
  (`AbilityTask_PlayMontageAndWait.CreatePlayMontageAndWaitProxy` "None" _montage 1.0 "None" false
    (:`then`
      (`AbilityTask_WaitGameplayEvent.WaitGameplayEvent` _montagetag null
        (:`EventReceived`
          (bind _returnvalue_6 (message `CombatInterface.GetCombatSocketLocation` _returnvalue_2 _sockettag))
          (set `self.SocketLocation` _returnvalue_6)
          (`KismetSystemLibrary.DrawDebugSphere` _returnvalue_6 50.0 12 (struct :`R` 0.009047 :`G` 1.0 :`B` 0.072751 :`A` 1.0) 3.0)
          (bind _outoverlappingactors (`AuraAbilitySystemLibrary.GetLivePlayersWithinRadius` _returnvalue_2 (`|MakeArray` _returnvalue_2) 100.0 _returnvalue_6))
          (for _array_element _outoverlappingactors
            (if (`AuraAbilitySystemLibrary.IsNotFriend` (`self.GetAvatarActorFromActorInfo`) _array_element)
              (`self.CauseDamage` _array_element)
              (set `self.HasHitTarget` true)))
          (if (`self.HasHitTarget`)
            (bind _returnvalue_7 (message `EnemyInterface.GetCombatTarget` (`self.GetAvatarActorFromActorInfo`)))
            (`self.K2_ExecuteGameplayCueWithParams` (struct :`TagName` "GameplayCue.MeleeAttack") (`AbilitySystemBlueprintLibrary.MakeGameplayCueParameters` 0.0 0.0 (struct) (struct) (struct) (`BlueprintGameplayTagLibrary.MakeGameplayTagContainerFromTag` (`.MontageTag` (break `TaggedMontage` (`self.TagMontage`)))) (struct) (`self.SocketLocation`) (0.0 0.0 0.0) null (`self.GetAvatarActorFromActorInfo`) _returnvalue_7)))
          (`self.K2_EndAbility`))))
    (:`OnCompleted`
      (`self.K2_EndAbility` :!label _label))
    (:`OnInterrupted`
      (goto _label))
    (:`OnCancelled`
      (goto _label))))