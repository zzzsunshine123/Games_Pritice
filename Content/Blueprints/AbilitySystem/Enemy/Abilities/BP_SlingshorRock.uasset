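; BP_SlingshorRock is the rock actor for an enemy slingshot ability, adding a random tumbling spin to its mesh.
; BeginPlay picks random yaw, pitch and roll rates, in either direction.
; Tick applies those rates, scaled by delta time, as local rotation on RockMesh.
; The Blueprint's own graphs contain no movement, overlap or damage logic.
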(event `self.ReceiveBeginPlay`
  (bind _returnvalue (`KismetMathLibrary.RandomFloatInRange` -500.0 500.0))
  (set `self.Yaw Rotation Rate` _returnvalue)
  (set `self.PitchRotation Rate` _returnvalue)
  (set `self.RollRotation Rate` _returnvalue))

(event `self.ReceiveTick`
  (params (DeltaSeconds :type "Float (single-precision)"))
  (`SceneComponent.K2_AddLocalRotation` (`self.RockMesh`) (`KismetMathLibrary.MakeRotator` (* DeltaSeconds (`self.RollRotation Rate`)) (* DeltaSeconds (`self.PitchRotation Rate`)) (* DeltaSeconds (`self.Yaw Rotation Rate`))) false false))

(fn `UserConstructionScript`)