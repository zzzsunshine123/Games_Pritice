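; Enemy gameplay ability that performs a ranged attack, firing a projectile at the avatar's combat target.
; On activation it stores the target's location, turns the avatar toward it and plays a random tagged attack montage.
; The montage's gameplay event tag triggers the projectile spawn from the tagged socket toward the stored location.
; The ability ends shortly after spawning, or when the montage completes, is interrupted or is cancelled.
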(event `self.K2_ActivateAbility`
  (bind _returnvalue (`self.GetAvatarActorFromActorInfo`))
  (bind _returnvalue_2 (message `EnemyInterface.GetCombatTarget` _returnvalue))
  (bind _returnvalue_3 (`Actor.K2_GetActorLocation` _returnvalue_2))
  (set `self.Projectile Target Location` _returnvalue_3)
  (message `CombatInterface.UpdateFacingTarget` _returnvalue _returnvalue_3)
  (bind _returnvalue_4 (message `CombatInterface.GetAttackMontages` (`self.GetAvatarActorFromActorInfo`)))
  (bind (_montage _montagetag _sockettag) (break `TaggedMontage` (`self.GetRandomTaggedMontageFromArray` _returnvalue_4)))
  (`AbilityTask_PlayMontageAndWait.CreatePlayMontageAndWaitProxy` "None" _montage
    (:`then`
      (`AbilityTask_WaitGameplayEvent.WaitGameplayEvent` _montagetag null true
        (:`EventReceived`
          (`self.SpawnProjectile` (`self.Projectile Target Location`) _sockettag (`self.Override Pitch`) (`self.Pitch Override`))
          (`KismetSystemLibrary.Delay` 0.5)
          (`self.K2_EndAbility`))))
    (:`OnCompleted`
      (`self.K2_EndAbility` :!label _label))
    (:`OnInterrupted`
      (goto _label))
    (:`OnCancelled`
      (goto _label))))